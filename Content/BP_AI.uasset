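; BP_AI is an AI character Blueprint with a squad-based color and a randomized movement speed.
; On BeginPlay it applies a blue or green AnimSharing material, selected by SquadNum, to the first two mesh slots and randomizes its max walk speed.
; It also holds an empty placeholder function and a macro that wraps PlayMontage on the mesh.
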(event EventBeginPlay
  (|CallParentFunction)
  (CallFunction|SetUpMaterial)
  (Variables|/Script/Engine.CharacterMovementComponent|SetMaxWalkSpeed (Variables|Character|GetCharacterMovement) (Math|Random|RandomFloatinRange 5e+02 1e+03)))

(fn ConstructionScript
  (|CallParentFunction))

(fn GetMaterial
  (return (Utilities|Select :Index (Variables|Default|GetSquadNum) :Option%200 "/AnimationSharing/AnimSharingBlue.AnimSharingBlue" :Option%201 "/AnimationSharing/AnimSharingGreen.AnimSharingGreen")))

(fn SetUpMaterial
  (bind _returnvalue (CallFunction|GetMaterial))
  (Rendering|Material|SetMaterial (Variables|Character|GetMesh) 0 _returnvalue)
  (Rendering|Material|SetMaterial (Variables|Character|GetMesh) 1 _returnvalue))

(fn Function
  (params (NewParam :type String)))